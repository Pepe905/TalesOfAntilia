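; Test Blueprint for Kanzar AI that makes the pawn wander around on its own.
; While it is not moving, Tick calls KanzarRoam, which waits a random few seconds, then picks a reachable point in a radius around its current location.
; AI MoveTo drives the walk, with IsMoving set during the move and cleared on success or failure so the next roam can begin.
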(event Custom|Kanzar%20Roam
  ;[0 0 0 0] Kanzar Roam
  (Utilities|FlowControl|Delay (Math|Random|RandomFloatinRange 5.0 1e+01))
  (Variables|Default|SetIs%20Moving? true)
  (bind _output_get (Variables|Default|SetRandom%20Location (.RandomLocation (AI|Navigation|GetRandomReachablePointinRadius (Transformation|GetActorLocation) 2e+03 0 0))))
  (AI|AIMoveTo self _output_get 0 5.0 false
    (:OnSuccess
      _)
    (:OnFail
      _))
  (Variables|Default|SetIs%20Moving? false))

(event EventBeginPlay)

(event Collision|EventActorBeginOverlap
  (params (OtherActor :type Actor%20Object%20Reference)))

(event EventTick
  (params (DeltaSeconds :type Float%20%28single-precision%29))
  ;[0 0 0.009721] Every Event Tick
  (Utilities|FlowControl|Sequence
    (:then_1
      (if (not (Variables|Default|GetIs%20Moving?))
        (CallFunction|KanzarRoam)))))

(fn ConstructionScript)