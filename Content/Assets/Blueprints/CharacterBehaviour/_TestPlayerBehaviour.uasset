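; Test VR player character with stick locomotion, speed change, two-hand grabbing, teleporting and a lightning spell.
; Grabs message overlapping interface actors; teleport traces a projectile path on press and moves only if the right trigger is held.
; Tick shows a PipBoy-style menu when it and the camera face each other, clicked through right-hand widget interaction.
; Spline-mesh teleport arc functions exist but are never called; the active trace uses debug drawing.
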(event EventTick
  (params (DeltaSeconds :type Float%20%28single-precision%29))
  ;[0.001887 0 0.09896] Teleportation Right Hand
  (Utilities|FlowControl|Sequence
    (:then_1
      ;[0.001821 0 0.0999] PipBoy - Menu Visibility
      (bind _returnvalue (CallFunction|DetectPipBoyDirection))
      (if _returnvalue
        (Rendering|SetVisibility (Variables|Default|GetWidget) true true)
        (Variables|/Script/UMG.WidgetInteractionComponent|SetbShowDebug (Variables|Default|GetWidgetInteractionRight) true)
        (else
          (Rendering|SetVisibility (Variables|Default|GetWidget) false true)
          (Variables|/Script/UMG.WidgetInteractionComponent|SetbShowDebug (Variables|Default|GetWidgetInteractionRight) false))))))

(event Input|ActionEvents|InputActionTeleportRight
  (params (Key :type Key%20Structure :default "None"))
  ;[0.001887 0 0.09896] Teleportation Right Hand
  (:Pressed
    (Utilities|FlowControl|Sequence
      (:then_0
        (Variables|Default|SetTeleportWish true))
      (:then_1
        (CallFunction|TraceforTeleport)
        (if (and (Variables|Default|GetCanTeleport) (Variables|Default|GetTriggerRightKeyPressed))
          (Transformation|Teleport (Variables|Default|GetTeleportDestination) (Transformation|GetWorldRotation (Variables|Default|GetMainCamera)))))))
  (:Released
    (Variables|Default|SetTeleportWish false)))

(event Input|ActionEvents|InputActionButtonY
  (params (Key :type Key%20Structure :default "None"))
  (bind _magicspawner (Variables|Default|GetMagicSpawner))
  (bind _returnvalue (Transformation|GetWorldTransform _magicspawner))
  ;[1 1 1] LightningSpell - Button Y
  (:Pressed
    (Game|SpawnActorfromClass "/Game/Marcel/Magic/LightningSpell.LightningSpell_C" (Math|Transform|MakeTransform (.location _returnvalue) (.rotation _returnvalue) "1.000000,1.000000,1.000000") "Undefined" 0 0)))

(event Input|ActionEvents|InputActionTriggerRight
  (params (Key :type Key%20Structure :default "None"))
  ;[0.001887 0 0.09896] Teleportation Right Hand
  (:Pressed
    (Variables|Default|SetTriggerRightKeyPressed true))
  (:Released
    (Variables|Default|SetTriggerRightKeyPressed false)))

(event Input|ActionEvents|InputActionGrabRight
  (params (Key :type Key%20Structure :default "None"))
  ;[0.001821 0 0.0999] Grab - Left and Right Controller
  (:Pressed
    (for _array_element (Collision|GetOverlappingActors (Variables|Default|GetSphereRight) 0 :!class /Script/Engine.PrimitiveComponent)
      (if (Utilities|DoesObjectImplementInterface _array_element 0)
        (Class|GrippableInterface|Grab(Message) _array_element (Variables|Default|GetMotionControllerRight))
        (Variables|Default|SetGrabRightActor _array_element))))
  (:Released
    (Utilities|IsValid (Variables|Default|GetGrabRightActor)
      (:Is%20Valid
        (Class|GrippableInterface|Release(Message) (Variables|Default|GetGrabRightActor))))))

(event Input|ActionEvents|InputActionGrabLeft
  (params (Key :type Key%20Structure :default "None"))
  ;[0.001821 0 0.0999] Grab - Left and Right Controller
  (:Pressed
    (for _array_element (Collision|GetOverlappingActors (Variables|Default|GetSphereLeft) 0 :!class /Script/Engine.PrimitiveComponent)
      (if (Utilities|DoesObjectImplementInterface _array_element 0)
        (Class|GrippableInterface|Grab(Message) _array_element (Variables|Default|GetMotionControllerLeft))
        (Variables|Default|SetGrabLeftActor _array_element))))
  (:Released
    (Utilities|IsValid (Variables|Default|GetGrabLeftActor)
      (:Is%20Valid
        (Class|GrippableInterface|Release(Message) (Variables|Default|GetGrabLeftActor))))))

(event Input|ActionEvents|InputActionTriggerRight
  (params (Key :type Key%20Structure :default "None"))
  (bind _widgetinteractionright (Variables|Default|GetWidgetInteractionRight))
  ;[0.001821 0 0.0999] Widget Interaction - Right Hand
  (:Pressed
    (Class|WidgetInteractionComponent|PressPointerKey _widgetinteractionright "LeftMouseButton"))
  (:Released
    (Class|WidgetInteractionComponent|ReleasePointerKey _widgetinteractionright "LeftMouseButton")))

(event Input|ActionEvents|InputActionTriggerLeft
  (params (Key :type Key%20Structure :default "None"))
  (bind _capsulecomponent (Variables|Collision|GetCapsuleComponent))
  (bind _returnvalue (Components|GetOwner _capsulecomponent))
  (bind _returnvalue_2 (Transformation|GetVelocity _returnvalue))
  ;[1 0 0] SPRINT
  (:Pressed
    (if (or (> (.x _returnvalue_2) 0.0) (> (.y _returnvalue_2) 0.0))
      (Variables|Default|SetSpeed 2e+01)
      (else
        (Variables|Default|SetSpeed 5.0))))
  (:Released
    (Variables|Default|SetSpeed 1e+01)))

(event Input|AxisEvents|InputAxisMovementAxisLeft_X
  (params (AxisValue :type Float%20%28single-precision%29))
  ;[0.001821 0 0.0999] Locomotion - Left Controller
  (Transformation|AddActorWorldOffset (* (Math|Vector|ProjectVectorontoPlane (Math|Vector|GetRightVector (Variables|Default|GetMainCamera)) "0, 0, 0") (* (Variables|Default|GetSpeed) AxisValue))))

(event Input|AxisEvents|InputAxisMovementAxisLeft_Y
  (params (AxisValue :type Float%20%28single-precision%29))
  ;[0.001821 0 0.0999] Locomotion - Left Controller
  (Transformation|AddActorWorldOffset (* (Math|Vector|ProjectVectorontoPlane (Math|Vector|GetForwardVector (Variables|Default|GetMainCamera)) "0, 0, 0") (* (Variables|Default|GetSpeed) AxisValue))))

(fn ConstructionScript)

(fn TeleportArc
  (params (StartingLocation :type Vector) (ForwardVector :type Vector))
  (bind _splinemeshes (Variables|Default|GetSplineMeshes))
  (bind _maincamera (Variables|Default|GetMainCamera))
  (bind _relativelocation (Variables|/Script/Engine.SceneComponent|GetRelativeLocation _maincamera))
  (bind (_outhit _outpathpositions _outlasttracedestination _returnvalue) (Class|GameplayStatics|BlueprintPredictProjectilePathbyTraceChannel StartingLocation (* ForwardVector (LocalVariables|GetForwardForce)) true 0.0 "ECC_WorldStatic" false 0 "None"))
  (LocalVariables|SetPaths _outpathpositions)
  (for _array_element _splinemeshes
    (Components|DestroyComponent _array_element)
    (for _index (range 0 (- (Utilities|Array|Length (LocalVariables|GetPaths)) 1))
      (bind _returnvalue_2 (AddComponent|AddSplineMeshComponent true))
      (Utilities|Array|Add (Variables|Default|GetSplineMeshes) 0)
      (SplineMesh|SetStartandEnd _returnvalue_2 (Utilities|Array|Get(acopy) (LocalVariables|GetPaths) (- _index 1)) "0, 0, 0" (Utilities|Array|Get(acopy) (LocalVariables|GetPaths) _index) "0, 0, 0" true :!class /Script/Engine.SplineMeshComponent))
    (if _returnvalue
      (if (.ReturnValue (AI|Navigation|ProjectPointtoNavigation _outlasttracedestination 0 0 "0, 0, 0"))
        (Variables|Default|SetTeleportLocation (Math|Vector|MakeVector (- (.x (.ProjectedLocation (AI|Navigation|ProjectPointtoNavigation _outlasttracedestination 0 0 "0, 0, 0"))) (.x _relativelocation)) (- (.y (.ProjectedLocation (AI|Navigation|ProjectPointtoNavigation _outlasttracedestination 0 0 "0, 0, 0"))) (.y _relativelocation)) (.z (.ProjectedLocation (AI|Navigation|ProjectPointtoNavigation _outlasttracedestination 0 0 "0, 0, 0")))))
        (else
          (Variables|Default|SetTeleportLocation (Transformation|GetActorLocation))))
      (else
        (Variables|Default|SetTeleportLocation (Transformation|GetActorLocation)))))
  (Utilities|Array|Clear _splinemeshes))

(fn ClearTeleportArc
  (bind _splinemeshes (Variables|Default|GetSplineMeshes))
  (for _array_element _splinemeshes
    (Components|DestroyComponent _array_element))
  (Utilities|Array|Clear _splinemeshes))

(fn DetectPipBoyDirection
  (bind _maincamera (Variables|Default|GetMainCamera))
  (bind _pipboyarrow (Variables|Default|GetPipBoyArrow))
  (return (and (Utilities|Operators|EqualEqual (Math|Vector|GetForwardVector _pipboyarrow) (Math|Vector|GetForwardVector (Math|Rotator|FindLookatRotation (Transformation|GetWorldLocation _pipboyarrow) (Transformation|GetWorldLocation (Variables|Default|GetMainCamera)))) 0.2) (Utilities|Operators|EqualEqual (Math|Vector|GetForwardVector _maincamera) (Math|Vector|GetForwardVector (Math|Rotator|FindLookatRotation (Transformation|GetWorldLocation _maincamera) (Transformation|GetWorldLocation (Variables|Default|GetPipBoyArrow)))) 0.5))))

(fn TraceforTeleport
  (bind _motioncontrollerright (Variables|Default|GetMotionControllerRight))
  (bind (_outhit _outpathpositions _outlasttracedestination _returnvalue) (Class|GameplayStatics|BlueprintPredictProjectilePathbyObjectType (Transformation|GetWorldLocation _motioncontrollerright) (* (Math|Vector|GetForwardVector (Transformation|GetWorldRotation _motioncontrollerright)) (Variables|Default|GetTelepotTraceLength)) true 5.0 (Utilities|Array|MakeArray "ObjectTypeQuery1") false 0 "ForOneFrame" 1.0 2.0))
  (if _returnvalue
    (Variables|Default|SetCanTeleport (> (.Z (Math|Vector|BreakVector (.ImpactNormal (Collision|BreakHitResult _outhit)))) 0.1))
    (bind _output_get (Variables|Default|SetTeleportDestination (.ImpactPoint (Collision|BreakHitResult _outhit))))
    (Class|KismetSystemLibrary|DrawDebugCylinder "0, 0, 0" (+ _output_get "0,0,50.000000") 5e+01 72 "(R=1.000000,G=0.145770,B=0.892244,A=0.495000)" 0.0 0.0)))