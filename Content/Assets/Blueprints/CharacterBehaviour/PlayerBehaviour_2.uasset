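; VR player Blueprint handling stick locomotion, speed changes, two-handed grabbing, teleportation, a wrist PipBoy menu and lightning spell spawning.
; Camera-relative axes offset the actor, and hand spheres send interface grab and release messages to overlapping objects.
; Holding teleport traces a debug-drawn projectile arc each tick, validating landings by surface normal for release.
; Mutual facing of wrist and camera reveals the PipBoy, with right-trigger widget clicks.
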(event EventTick
  (params (DeltaSeconds :type Float%20%28single-precision%29))
  ;[0.001887 0 0.09896] Teleportation Right Hand
  (Utilities|FlowControl|Sequence
    (:then_0
      (if (Variables|Default|GetTeleportKeyPress)
        (CallFunction|TraceforTeleportation)))
    (:then_1
      ;[0.001821 0 0.0999] PipBoy - Menu Visibility
      (bind _returnvalue (CallFunction|DetectPipBoyDirection))
      (if _returnvalue
        (Rendering|SetVisibility (Variables|Default|Get_WidgetPipBoy) true true)
        (Variables|/Script/UMG.WidgetInteractionComponent|SetbShowDebug (Variables|Default|GetWidgetInteractionRight) true)
        (else
          (Rendering|SetVisibility (Variables|Default|Get_WidgetPipBoy) false true)
          (Variables|/Script/UMG.WidgetInteractionComponent|SetbShowDebug (Variables|Default|GetWidgetInteractionRight) false))))))

(event Input|ActionEvents|InputActionTeleportRight
  (params (Key :type Key%20Structure :default "None"))
  ;[0.001887 0 0.09896] Teleportation Right Hand
  (:Pressed
    (Variables|Default|SetTeleportKeyPress true))
  (:Released
    (Variables|Default|SetTeleportKeyPress false)
    (Development|SetHiddeninGame (Variables|Default|GetTeleportationArrow) true false)
    (if (Variables|Default|GetCanTeleport)
      (Transformation|Teleport (Variables|Default|GetTeleportLocation) (Transformation|GetActorRotation)))))

(event Input|ActionEvents|InputActionButtonB
  (params (Key :type Key%20Structure :default "None"))
  (bind _magicspawner (Variables|Default|GetMagicSpawner))
  (bind _returnvalue (Transformation|GetWorldTransform _magicspawner))
  ;[1 1 1] LightningSpell - Button Y
  (:Pressed
    (Game|SpawnActorfromClass "/Game/Marcel/Magic/LightningSpell.LightningSpell_C" (Math|Transform|MakeTransform (.location _returnvalue) (.rotation _returnvalue) "1.000000,1.000000,1.000000") "Undefined" 0 0)))

(event Input|ActionEvents|InputActionGrabRight
  (params (Key :type Key%20Structure :default "None"))
  ;[0.001821 0 0.0999] Grab - Left and Right Controller
  (:Pressed
    (for _array_element (Collision|GetOverlappingActors (Variables|Pawn|GetSphereRight) 0 :!class /Script/Engine.PrimitiveComponent)
      (if (Utilities|DoesObjectImplementInterface _array_element 0)
        (Class|GrippableInterface|Grab(Message) _array_element (Variables|Default|GetMotionControllerRight))
        (Variables|Default|SetGrabRightActor _array_element))))
  (:Released
    (Utilities|IsValid (Variables|Default|GetGrabRightActor)
      (:Is%20Valid
        (Class|GrippableInterface|Release(Message) (Variables|Default|GetGrabRightActor))))))

(event Input|ActionEvents|InputActionGrabLeft
  (params (Key :type Key%20Structure :default "None"))
  ;[0.001821 0 0.0999] Grab - Left and Right Controller
  (:Pressed
    (for _array_element (Collision|GetOverlappingActors (Variables|Default|GetSphereLeft) 0 :!class /Script/Engine.PrimitiveComponent)
      (if (Utilities|DoesObjectImplementInterface _array_element 0)
        (Class|GrippableInterface|Grab(Message) _array_element (Variables|Default|GetMotionControllerLeft))
        (Variables|Default|SetGrabLeftActor _array_element))))
  (:Released
    (Utilities|IsValid (Variables|Default|GetGrabLeftActor)
      (:Is%20Valid
        (Class|GrippableInterface|Release(Message) (Variables|Default|GetGrabLeftActor))))))

(event Input|ActionEvents|InputActionTriggerRight
  (params (Key :type Key%20Structure :default "None"))
  (bind _widgetinteractionright (Variables|Default|GetWidgetInteractionRight))
  ;[0.001821 0 0.0999] Widget Interaction - Right Hand
  (:Pressed
    (Class|WidgetInteractionComponent|PressPointerKey _widgetinteractionright "LeftMouseButton"))
  (:Released
    (Class|WidgetInteractionComponent|ReleasePointerKey _widgetinteractionright "LeftMouseButton")))

(event Input|ActionEvents|InputActionTriggerLeft
  (params (Key :type Key%20Structure :default "None"))
  (bind _returnvalue (Transformation|GetVelocity))
  ;[1 0 0] SPRINT
  (:Pressed
    (if (or (!= (.x _returnvalue) 0.0) (!= (.y _returnvalue) 0.0))
      (Variables|Default|SetSpeed 2e+01)
      (else
        (Variables|Default|SetSpeed 5.0))))
  (:Released
    (Variables|Default|SetSpeed 1e+01)))

(event Input|AxisEvents|InputAxisMovementAxisLeft_Y
  (params (AxisValue :type Float%20%28single-precision%29))
  ;[0.001821 0 0.0999] Locomotion - Left Controller
  (Transformation|AddActorWorldOffset (* (Math|Vector|ProjectVectorontoPlane (Math|Vector|GetForwardVector (Variables|Default|GetMainCamera)) "0, 0, 0") (* (Variables|Default|GetSpeed) AxisValue))))

(event Input|AxisEvents|InputAxisMovementAxisLeft_X
  (params (AxisValue :type Float%20%28single-precision%29))
  ;[0.001821 0 0.0999] Locomotion - Left Controller
  (Transformation|AddActorWorldOffset (* (Math|Vector|ProjectVectorontoPlane (Math|Vector|GetRightVector (Variables|Default|GetMainCamera)) "0, 0, 0") (* (Variables|Default|GetSpeed) AxisValue))))

(fn ConstructionScript)

(fn DetectPipBoyDirection
  (bind _maincamera (Variables|Default|GetMainCamera))
  (bind _pipboyarrow (Variables|Default|GetPipBoyArrow))
  (return (and (Utilities|Operators|EqualEqual (Math|Vector|GetForwardVector _pipboyarrow) (Math|Vector|GetForwardVector (Math|Rotator|FindLookatRotation (Transformation|GetWorldLocation _pipboyarrow) (Transformation|GetWorldLocation (Variables|Default|GetMainCamera)))) 0.2) (Utilities|Operators|EqualEqual (Math|Vector|GetForwardVector _maincamera) (Math|Vector|GetForwardVector (Math|Rotator|FindLookatRotation (Transformation|GetWorldLocation _maincamera) (Transformation|GetWorldLocation (Variables|Default|GetPipBoyArrow)))) 0.5))))

(fn TraceforTeleportation
  (bind _motioncontrollerright (Variables|Default|GetMotionControllerRight))
  (bind _teleportationarrow (Variables|Default|GetTeleportationArrow))
  (bind (_outhit _outpathpositions _outlasttracedestination _returnvalue) (Class|GameplayStatics|BlueprintPredictProjectilePathbyObjectType (Transformation|GetWorldLocation _motioncontrollerright) (* (Math|Vector|GetForwardVector (Transformation|GetWorldRotation _motioncontrollerright)) (Variables|Default|GetTeleportationTraceLength)) true 1e+01 (Utilities|Array|MakeArray "ObjectTypeQuery1" "ObjectTypeQuery2") false 0 "ForOneFrame" 0.0 2e+01))
  (if _returnvalue
    (Variables|Default|SetCanTeleport (> (.Z (Math|Vector|BreakVector (.ImpactNormal (Collision|BreakHitResult _outhit)))) 0.1))
    (bind _output_get (Variables|Default|SetTeleportLocation (.ImpactPoint (Collision|BreakHitResult _outhit))))
    (Class|KismetSystemLibrary|DrawDebugCylinder _output_get (+ _output_get "0,0,20.000000") 5e+01 20 "(R=1.000000,G=0.000000,B=0.830346,A=1.000000)" 0.0 0.0)
    (Development|SetHiddeninGame _teleportationarrow false false)
    (Transformation|SetWorldLocation _teleportationarrow (Variables|Default|GetTeleportLocation) false false)
    (else
      (Development|SetHiddeninGame (Variables|Default|GetTeleportationArrow) true false))))