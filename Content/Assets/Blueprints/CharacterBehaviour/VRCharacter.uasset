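; VR player character that handles two-handed grabbing, smooth locomotion and UI interaction through motion controllers.
; Grab inputs send GrabMessage with the hand's controller to every GrippableInterface actor overlapping that hand's sphere, storing only the last for release.
; Left-hand axes drive movement along the left controller's forward and right vectors.
; Triggers press and release each hand's WidgetInteraction pointer as a left mouse click.
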(event Input|ActionEvents|InputActionGrabLeft
  (params (Key :type Key%20Structure :default "None"))
  ;[0.08333 0.08333 0.08333] Locomotion Movement
  (:Pressed
    (for _array_element (Collision|GetOverlappingActors (Variables|Default|GetSphereLeft) 0 :!class /Script/Engine.PrimitiveComponent)
      (if (Utilities|DoesObjectImplementInterface _array_element "/Game/Assets/Blueprints/CharacterBehaviour/GrippableInterface.GrippableInterface_C")
        (Class|GrippableInterface|Grab(Message) _array_element (Variables|Default|GetMotionControllerLeft))
        (Variables|Default|SetGrabLeftActor _array_element))))
  (:Released
    (Utilities|IsValid (Variables|Default|GetGrabLeftActor)
      (:Is%20Valid
        (Class|GrippableInterface|Release(Message) (Variables|Default|GetGrabLeftActor))))))

(event Input|ActionEvents|InputActionGrabRight
  (params (Key :type Key%20Structure :default "None"))
  ;[0.08333 0.08333 0.08333] Locomotion Movement
  (:Pressed
    (for _array_element (Collision|GetOverlappingActors (Variables|Default|GetSphereRight) 0 :!class /Script/Engine.PrimitiveComponent)
      (if (Utilities|DoesObjectImplementInterface _array_element "/Game/Assets/Blueprints/CharacterBehaviour/GrippableInterface.GrippableInterface_C")
        (Class|GrippableInterface|Grab(Message) _array_element (Variables|Default|GetMotionControllerRight))
        (Variables|Default|SetGrabRightActor _array_element))))
  (:Released
    (Utilities|IsValid (Variables|Default|GetGrabRightActor)
      (:Is%20Valid
        (Class|GrippableInterface|Release(Message) (Variables|Default|GetGrabRightActor))))))

(event Input|ActionEvents|InputActionTriggerLeft
  (params (Key :type Key%20Structure :default "None"))
  (bind _widgetinteractionleft (Variables|Default|GetWidgetInteractionLeft))
  ;[1 1 1] Widget Interaction Both Hands
  (:Pressed
    (Class|WidgetInteractionComponent|PressPointerKey _widgetinteractionleft "LeftMouseButton"))
  (:Released
    (Class|WidgetInteractionComponent|ReleasePointerKey _widgetinteractionleft "LeftMouseButton")))

(event Input|ActionEvents|InputActionTriggerRight
  (params (Key :type Key%20Structure :default "None"))
  (bind _widgetinteractionright (Variables|Default|GetWidgetInteractionRight))
  ;[1 1 1] Widget Interaction Both Hands
  (:Pressed
    (Class|WidgetInteractionComponent|PressPointerKey _widgetinteractionright "LeftMouseButton"))
  (:Released
    (Class|WidgetInteractionComponent|ReleasePointerKey _widgetinteractionright "LeftMouseButton")))

(event Input|AxisEvents|InputAxisMovementAxisLeft_X
  (params (AxisValue :type Float%20%28single-precision%29))
  ;[0.08333 0.08333 0.08333] Locomotion Movement
  (Pawn|Input|AddMovementInput (Math|Vector|GetRightVector (Variables|Default|GetMotionControllerLeft)) AxisValue false))

(event Input|AxisEvents|InputAxisMovementAxisLeft_Y
  (params (AxisValue :type Float%20%28single-precision%29))
  ;[0.08333 0.08333 0.08333] Locomotion Movement
  (Pawn|Input|AddMovementInput (Math|Vector|GetForwardVector (Variables|Default|GetMotionControllerLeft)) AxisValue false))

(fn ConstructionScript)