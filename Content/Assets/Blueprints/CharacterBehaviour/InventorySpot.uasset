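; VR inventory slot collision component that snaps a released ItemPrefabBlanko item onto itself.
; Each tick, a valid GrabActor with no valid MotionController is attached to the spot, keeping world scale.
; Ending overlap with that actor clears GrabActor.
; Begin overlap checks for a held item when the slot is empty but takes no action, so nothing here assigns GrabActor.
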(event Custom|BeginOverlap
  (params (OverlappedComponent :type Primitive%20Component%20Object%20Reference) (OtherActor :type Actor%20Object%20Reference) (OtherComp :type Primitive%20Component%20Object%20Reference) (OtherBodyIndex :type Integer) (bFromSweep :type Boolean) (SweepResult :type Hit%20Result%20Structure%20%28by%20ref%29))
  (Utilities|IsValid (Variables|Default|GetGrabActor)
    (:Is%20Not%20Valid
      (bind _asitem_prefab_blanko (Utilities|Casting|CastToItemPrefabBlanko OtherActor))
      (Utilities|IsValid (Variables|/Game/Assets/Blueprints/CharacterBehaviour/ItemPrefabBlanko.ItemPrefabBlanko_C|GetMotionController _asitem_prefab_blanko)))))

(event Custom|EndOverlap
  (params (OverlappedComponent :type Primitive%20Component%20Object%20Reference) (OtherActor :type Actor%20Object%20Reference) (OtherComp :type Primitive%20Component%20Object%20Reference) (OtherBodyIndex :type Integer))
  (if (== OtherActor (Variables|Default|GetGrabActor))
    (Variables|Default|SetGrabActor 0)))

(event EventBeginPlay
  (Collision|AssignOnComponentBeginOverlap (delegate Custom|BeginOverlap))
  (Collision|BindEventtoOnComponentEndOverlap (delegate Custom|EndOverlap)))

(event EventTick
  (params (DeltaSeconds :type Float%20%28single-precision%29))
  (bind _grabactor (Variables|Default|GetGrabActor))
  (Utilities|IsValid _grabactor
    (:Is%20Valid
      (Utilities|IsValid (Variables|/Game/Assets/Blueprints/CharacterBehaviour/ItemPrefabBlanko.ItemPrefabBlanko_C|GetMotionController _grabactor)
        (:Is%20Not%20Valid
          (Transformation|AttachComponentToComponent _grabactor self "None" "SnapToTarget" "SnapToTarget" "KeepWorld" true))))))