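; BP_EnemyTest is a test enemy Blueprint that turns an Enemy reference toward a Target while its sphere trigger is occupied.
; Sphere begin and end overlaps toggle IsInside without filtering the overlapping actor.
; While the flag is set, Tick smoothly rotates Enemy with RInterpTo and FindLookAtRotation.
; The same chain runs through a ten-second Delay, so a Niagara component is added repeatedly at roughly that interval.
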(event OnComponentBeginOverlap(Sphere)
  (params (OverlappedComponent :type Primitive%20Component%20Object%20Reference) (OtherActor :type Actor%20Object%20Reference) (OtherComp :type Primitive%20Component%20Object%20Reference) (OtherBodyIndex :type Integer) (bFromSweep :type Boolean) (SweepResult :type Hit%20Result%20Structure%20%28by%20ref%29))
  (Variables|Default|SetIsInside true))

(event OnComponentEndOverlap(Sphere)
  (params (OverlappedComponent :type Primitive%20Component%20Object%20Reference) (OtherActor :type Actor%20Object%20Reference) (OtherComp :type Primitive%20Component%20Object%20Reference) (OtherBodyIndex :type Integer))
  (Variables|Default|SetIsInside false))

(event EventTick
  (params (DeltaSeconds :type Float%20%28single-precision%29))
  (bind _enemy (Variables|Default|GetEnemy))
  (if (Variables|Default|GetIsInside)
    (Transformation|SetWorldRotation (Variables|/Script/Engine.Actor|GetRootComponent _enemy) (Math|Interpolation|RInterpTo (Transformation|GetWorldRotation (Variables|/Script/Engine.Actor|GetRootComponent _enemy)) (Math|Rotator|FindLookatRotation (Transformation|GetWorldLocation (Variables|/Script/Engine.Actor|GetRootComponent _enemy)) (Transformation|GetWorldLocation (Variables|/Script/Engine.Actor|GetRootComponent (Variables|Default|GetTarget)))) (Utilities|Time|GetWorldDeltaSeconds) 1.0) false false)
    (Utilities|FlowControl|Delay 1e+01)
    (AddComponent|AddNiagaraComponent false)))

(fn ConstructionScript)