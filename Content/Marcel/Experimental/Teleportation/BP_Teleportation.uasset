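; BP_Teleportation is an experimental teleporter trigger that plays the start of a teleport effect, with no relocation logic implemented.
; A swept overlap on CollisionSensor resets Ported and stores the overlapping Viridium_Character as Creature.
; After short delays it calls a 2D sound, then applies a dynamic instance of Teleport_TestMat to the character's first mesh material slot.
; A node setting the character's IsMoving flag is left unconnected.
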(event OnComponentBeginOverlap(CollisionSensor)
  (params (OverlappedComponent :type Primitive%20Component%20Object%20Reference) (OtherActor :type Actor%20Object%20Reference) (OtherComp :type Primitive%20Component%20Object%20Reference) (OtherBodyIndex :type Integer) (bFromSweep :type Boolean) (SweepResult :type Hit%20Result%20Structure%20%28by%20ref%29))
  (if bFromSweep
    (Variables|Default|SetPorted false)
    (bind _asviridium_character (Utilities|Casting|CastToViridium_Character OtherActor))
    (bind _output_get (Variables|Default|SetCreature _asviridium_character))
    (Utilities|FlowControl|Sequence
      (:then_0
        (Utilities|FlowControl|Delay 0.5)
        (Audio|PlaySound2D 0 1.0 1.0 0.0 0 0)
        (Utilities|FlowControl|Delay 0.5)
        (Rendering|Material|CreateDynamicMaterialInstance (Variables|/Script/Engine.Character|GetMesh (Variables|Default|GetCreature)) 0 "/Game/Marcel/Experimental/Teleportation/Teleport_TestMat.Teleport_TestMat" "None" :!class /Script/Engine.PrimitiveComponent)))))

(fn ConstructionScript)