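; Catch spell actor that captures tagged creatures through a sphere overlap, then destroys itself.
; After a short delay, the creature tag selects which cage gets its teleported flag and which caught flag is set.
; Creatures One and Two also require ViridiumFree and OccamyFree respectively; only ViridiumFree is set here, on BeginPlay.
; Creature One's caught flag is written through the CreatureThreeCatched reference, and unmatched overlaps just destroy the actor.
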(event OnComponentBeginOverlap(Sphere)
  (params (OverlappedComponent :type Primitive%20Component%20Object%20Reference) (OtherActor :type Actor%20Object%20Reference) (OtherComp :type Primitive%20Component%20Object%20Reference) (OtherBodyIndex :type Integer) (bFromSweep :type Boolean) (SweepResult :type Hit%20Result%20Structure%20%28by%20ref%29))
  (Utilities|FlowControl|Delay 0.1)
  (if (and (Actor|ActorHasTag OtherActor "Creature_One") (Variables|Default|GetViridium_Free))
    (Variables|/Game/Marcel/Experimental/Teleportation/BP_Cage_One.BP_Cage_One_C|SetIsTeleported_One (Utilities|ResolveSoftReference (Variables|Default|GetCage_One)) true)
    (Variables|/Game/Marcel/Experimental/Creature_Manager.Creature_Manager_C|SetCreature_One_Catched (Utilities|ResolveSoftReference (Variables|Default|GetCreature_Three_Catched)) true)
    (Actor|DestroyActor :!label _label)
    (elif (and (Actor|ActorHasTag OtherActor "Creature_Two") (Variables|Default|GetOccamy_Free))
      (Variables|/Game/Marcel/Experimental/Teleportation/BP_Cage_Two.BP_Cage_Two_C|SetIsTeleported_Two (Utilities|ResolveSoftReference (Variables|Default|GetCage_Two)) true)
      (Variables|/Game/Marcel/Experimental/Creature_Manager.Creature_Manager_C|SetCreature_Two_Catched (Utilities|ResolveSoftReference (Variables|Default|GetCreature_Two_Catched)) true)
      (goto _label)
      (elif (Actor|ActorHasTag OtherActor "Creature_Three")
        (Variables|/Game/Marcel/Experimental/Teleportation/BP_Cage_Three.BP_Cage_Three_C|SetIsTeleported_Three (Utilities|ResolveSoftReference (Variables|Default|GetCage_Three)) true)
        (Variables|/Game/Marcel/Experimental/Creature_Manager.Creature_Manager_C|SetCreature_Three_Catched (Utilities|ResolveSoftReference (Variables|Default|GetCreature_Three_Catched)) true)
        (goto _label)
        (else
          (Actor|DestroyActor))))))

(event EventBeginPlay
  (Variables|Default|SetViridium_Free true))

(event Collision|EventActorBeginOverlap
  (params (OtherActor :type Actor%20Object%20Reference)))

(event EventTick
  (params (DeltaSeconds :type Float%20%28single-precision%29)))

(fn ConstructionScript)